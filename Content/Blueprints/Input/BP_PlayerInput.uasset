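; BP_PlayerInput gathers Enhanced Input actions into player input state variables.
; BeginPlay adds IMC_Default, then Tick passes the left stick to CalLeftStickInput for interpolation and polls right stick, jump and sprint values.
; IA_LockOn and IA_Dodge events handle the rest, with lock-on toggling on a true value and dodge mirroring its action value.
; Sprint and dodge values are printed to screen as debug output.
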(event EventBeginPlay
  (Input|AddMappingContext (PlayerController|LocalPlayerSubsystems|GetEnhancedInputLocalPlayerSubsystem) "/Game/Input/IMC_Default.IMC_Default" 0 "(bIgnoreAllPressedKeysUntilRelease=True,bForceImmediately=False,bNotifyUserSettings=False)"))

(event Input|EnhancedActionEvents|EnhancedInputActionIA_Dodge
  (params (ActionValue :type Boolean) (ElapsedSeconds :type Float%20%28double-precision%29) (TriggeredSeconds :type Float%20%28double-precision%29) (InputAction :type Input%20Action%20Object%20Reference :default "/Game/Input/Actions/IA_Dodge.IA_Dodge"))
  ;[1 1 1] Buttons
  (bind _output_get (Variables|Default|SetDodge ActionValue))
  (Development|PrintString (Utilities|String|ToString(Boolean) _output_get) true true "(R=1.000000,G=0.081270,B=0.000000,A=1.000000)"))

(event Input|EnhancedActionEvents|EnhancedInputActionIA_LockOn
  (params (ActionValue :type Boolean) (ElapsedSeconds :type Float%20%28double-precision%29) (TriggeredSeconds :type Float%20%28double-precision%29) (InputAction :type Input%20Action%20Object%20Reference :default "/Game/Input/Actions/IA_LockOn.IA_LockOn"))
  ;[1 1 1] Buttons
  (if ActionValue
    (Variables|Default|SetLockOn (not (Variables|Default|GetLockOn)))))

(event EventTick
  (params (DeltaSeconds :type Float%20%28single-precision%29))
  (bind _returnvalue (Input|EnhancedActionValues|GetIA_RightStick))
  (bind (_x _y) (Math|Vector2D|BreakVector2D _returnvalue))
  (Utilities|FlowControl|Sequence
    (:then_0
      ;[1 1 1] LeftStick
      (Class|PlayerInputManager|CalLeftStickInput (Input|EnhancedActionValues|GetIA_LeftStick) DeltaSeconds 5.0))
    (:then_1
      ;[1 1 1] RightStick
      (Variables|Default|SetJright _x)
      (Variables|Default|SetJup _y))
    (:then_2
      ;[1 1 1] Buttons
      (Variables|Default|SetJump (Input|EnhancedActionValues|GetIA_Jump)))
    (:then_3
      (bind _output_get (Variables|Default|SetSprint (Input|EnhancedActionValues|GetIA_Sprint)))
      (Development|PrintString (Utilities|String|ToString(Boolean) _output_get)))))

(fn ConstructionScript)