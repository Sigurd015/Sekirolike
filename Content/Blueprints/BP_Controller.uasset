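; BP_Controller turns Enhanced Input actions into state variables for locomotion and camera-style stick input, adding the keyboard mapping context on BeginPlay.
; CalLeftStickValue converts the left stick axis, actor forward and right vectors, and delta time into directional components, magnitude and vector.
; Right stick axes are stored raw, Jump stores and prints its value, and Lock toggles LockState when pressed.
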(event EventBeginPlay
  (Input|AddMappingContext (PlayerController|LocalPlayerSubsystems|GetEnhancedInputLocalPlayerSubsystem) "/Game/Input/IMC_Keyboard.IMC_Keyboard" 0 "(bIgnoreAllPressedKeysUntilRelease=True,bForceImmediately=False,bNotifyUserSettings=False)"))

(event Input|EnhancedActionEvents|EnhancedInputActionIA_LeftStick
  (params (ActionValue :type Vector%202D%20Structure) (ElapsedSeconds :type Float%20%28double-precision%29) (TriggeredSeconds :type Float%20%28double-precision%29) (InputAction :type Input%20Action%20Object%20Reference :default "/Game/Input/Actions/IA_LeftStick.IA_LeftStick"))
  ;[1 1 1] LeftStick
  (bind (_dup _dright _dmag _dvec) (Class|CalInputValue|CalLeftStickValue ActionValue (Transformation|GetActorForwardVector) (Transformation|GetActorRightVector) (Utilities|Time|GetWorldDeltaSeconds) 5.0))
  (Variables|Default|SetDup _dup)
  (Variables|Default|SetDright _dright)
  (Variables|Default|SetDmag _dmag)
  (Variables|Default|SetDvec _dvec))

(event Input|EnhancedActionEvents|EnhancedInputActionIA_RightStick
  (params (ActionValue :type Vector%202D%20Structure) (ElapsedSeconds :type Float%20%28double-precision%29) (TriggeredSeconds :type Float%20%28double-precision%29) (InputAction :type Input%20Action%20Object%20Reference :default "/Game/Input/Actions/IA_RightStick.IA_RightStick"))
  (bind (_x _y) (Math|Vector2D|BreakVector2D ActionValue))
  ;[1 1 1] RightStick
  (Variables|Default|SetJright _x)
  (Variables|Default|SetJup _y))

(event Input|EnhancedActionEvents|EnhancedInputActionIA_Jump
  (params (ActionValue :type Boolean) (ElapsedSeconds :type Float%20%28double-precision%29) (TriggeredSeconds :type Float%20%28double-precision%29) (InputAction :type Input%20Action%20Object%20Reference :default "/Game/Input/Actions/IA_Jump.IA_Jump"))
  ;[1 1 1] Buttons
  (bind _output_get (Variables|Default|SetJump ActionValue))
  (Development|PrintString (Utilities|String|ToString(Boolean) _output_get)))

(event Input|EnhancedActionEvents|EnhancedInputActionIA_Lock
  (params (ActionValue :type Boolean) (ElapsedSeconds :type Float%20%28double-precision%29) (TriggeredSeconds :type Float%20%28double-precision%29) (InputAction :type Input%20Action%20Object%20Reference :default "/Game/Input/Actions/IA_Lock.IA_Lock"))
  ;[1 1 1] Buttons
  (if ActionValue
    (Variables|Default|SetLockState (not (Variables|Default|GetLockState)))))

(fn ConstructionScript)